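; Double door actor that the player opens and closes with the E key while standing inside its Box trigger.
; Overlap begin and end toggle input; E plays sounds, then plays or reverses two timelines that yaw Door and Door2, based on Isclosed.
; Tick recomputes Isclosed from both timelines' rotation values, the second overwriting the first, and extra sounds play when movement finishes with the doors closed.
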(event `Key|E`
  (params (Key :type "Key Structure"))
  (bind _isclosed (`self.isclosed`))
  (:`Pressed`
    (`GameplayStatics.PlaySound2D` null 1.0 1.0 0.0 null null)
    (`GameplayStatics.PlaySound2D` null 1.0 1.0 0.0 null null)
    (`KismetSystemLibrary.Delay` 0.2)
    (`GameplayStatics.PlaySound2D` null 1.0 1.0 0.0 null null)
    (`|ExecutionSequence`
      (:`then_0`
        (if _isclosed
          (bind (_direction _rote) (`Timeline|DoorRote` :!label _label)
            (:`Update`
              (`SceneComponent.K2_SetRelativeRotation` (`self.Door`) (`KismetMathLibrary.MakeRotator` 0.0 0.0 _rote) false false))
            (:`Finished`
              (if _isclosed
                (`GameplayStatics.PlaySound2D` null 1.0 1.0 0.0 null null)
                (`KismetSystemLibrary.Delay` 0.1)
                (`GameplayStatics.PlaySound2D` null 1.0 1.0 0.0 null null))))
          (else
            (goto _label :!via `Reverse`))))
      (:`then_1`
        (if _isclosed
          (bind (_direction_2 _rote_2) (`Timeline|OtherDoorRote` :!label _label_2)
            (:`Update`
              (`SceneComponent.K2_SetRelativeRotation` (`self.Door2`) (`KismetMathLibrary.MakeRotator` 0.0 0.0 _rote_2) false false)))
          (else
            (goto _label_2 :!via `Reverse`)))))))

(event `self.Box.OnComponentBeginOverlap`
  (params (OverlappedComponent :type "PrimitiveComponent Object Reference") (OtherActor :type "Actor Object Reference") (OtherComp :type "PrimitiveComponent Object Reference") (OtherBodyIndex :type Integer) (bFromSweep :type Boolean) (SweepResult :type "HitResult Structure (by ref)"))
  (`self.EnableInput` (`GameplayStatics.GetPlayerController` 0)))

(event `self.ReceiveTick`
  (params (DeltaSeconds :type "Float (single-precision)"))
  (set `self.isclosed` (< (stale `Key|E` _rote) -1.0))
  (set `self.isclosed` (< (stale `Key|E` _rote_2) 1.0)))

(event `self.Box.OnComponentEndOverlap`
  (params (OverlappedComponent :type "PrimitiveComponent Object Reference") (OtherActor :type "Actor Object Reference") (OtherComp :type "PrimitiveComponent Object Reference") (OtherBodyIndex :type Integer))
  (`self.DisableInput` (`GameplayStatics.GetPlayerController` 0)))

(fn `UserConstructionScript`)