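; BP_SunRotation rotates the referenced sun actor to match game time and speed, keeping the sky sphere in sync.
; On BeginPlay it reads the game speed from BP_GameState and binds to its speed control event for updates.
; Each Tick, SetGameTime turns delta time, speed and the GameTime variable into a scaled local pitch increment for the sun, then the sky sphere's sun direction is refreshed.
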(event `self.ReceiveBeginPlay`
  (set `self.GameStateRef` (cast `/Game/MainAssets/Blueprints/Settings/BP_GameState` (`GameplayStatics.GetGameState`) :!pure true))
  (add `/Game/MainAssets/Blueprints/Settings/BP_GameState.GameSpeedControl` (`self.GameStateRef`) (`|CreateDelegate` :!event `GetGameSpeed`))
  (bind _gamespeed (`/Game/MainAssets/Blueprints/Settings/BP_GameState.GetGameSpeed` (`self.GameStateRef`)))
  (set `self.GameSpeed` _gamespeed))

(event `GetGameSpeed`
  (params (GameSpeed :type "Float (double-precision)"))
  (set `self.GameSpeed` GameSpeed))

(event `self.ReceiveTick`
  (params (DeltaSeconds :type "Float (single-precision)"))
  (`self.K2_AddActorLocalRotation` (`self.SunRef`) (`KismetMathLibrary.MakeRotator` 0.0 (* (/ (/ (`/Game/MainAssets/Blueprints/Libraries/BP_FuncLib.SetGameTime` DeltaSeconds (`self.GameSpeed`) (`self.GameTime`)) 1.5) 6.0) 90.0)) false false)
  (`/Engine/EngineSky/BP_Sky_Sphere.UpdateSunDirection` (`self.SkySphereRef`)))

(fn `UserConstructionScript`)