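; RTS camera pawn that moves, pans and zooms the view, adding a clock/calendar HUD when possessed.
; Axis input moves an invisible pivot mesh at a speed scaled by spring-arm length, with Shift boosting movement and screen-edge scrolling.
; Gates let mouse movement rotate the pivot while Pan is held, and let Tick spawn particles at the cursor trace hit while left mouse is held.
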(event `self.ReceivePossessed`
  (params (NewController :type "Controller Object Reference"))
  (`|ExecutionSequence`
    (:`then_0`
      (bind _asbp_game_state (cast `/Game/MainAssets/Blueprints/Settings/BP_GameState` (`GameplayStatics.GetGameState`)))
      (set `self.GameStateRef` _asbp_game_state))
    (:`then_1`
      (`self.SpawnWidgets`)
      (`UserWidget.AddToViewport` (`self.Hud_CNC_Ref`) 0))))

(event `self.ReceiveUnpossessed`
  (params (OldController :type "Controller Object Reference"))
  (`WidgetLayoutLibrary.RemoveAllWidgets`))

(event `InputAxis|MoveForward`
  (params (AxisValue :type "Float (single-precision)"))
  ;[1 1 1] Camera Movement
  (`SceneComponent.K2_SetWorldTransform` (`self.Invisible Mesh`) (`self.MovementX` (`self.MovementSpeedCalc`) (`self.FastMoveMult`) AxisValue "/Game/MainAssets/Characters/MainCharacter/BPs/Blueprints/InvisibleMesh.InvisibleMesh") false false))

(event `InputAction|Pan`
  (params (Key :type "Key Structure"))
  (bind _panspeed (`self.PanSpeed`))
  (bind _invisible_mesh (`self.Invisible Mesh`))
  ;[1 1 1] Panning and Edge Scroll
  (:`Pressed`
    (goto _label_2 :!via `Open`))
  (:`Released`
    (goto _label_2 :!via `Close`)))

(event `InputAxis|MoveRight`
  (params (AxisValue :type "Float (single-precision)"))
  ;[1 1 1] Camera Movement
  (`SceneComponent.K2_SetWorldTransform` (`self.Invisible Mesh`) (`KismetMathLibrary.MakeTransform` (`KismetMathLibrary.MakeVector` (.x (.location (`self.MovementY` (`self.MovementSpeedCalc`) (`self.FastMoveMult`) AxisValue "/Game/MainAssets/Characters/MainCharacter/BPs/Blueprints/InvisibleMesh.InvisibleMesh"))) (.y (.location (`self.MovementY` (`self.MovementSpeedCalc`) (`self.FastMoveMult`) AxisValue "/Game/MainAssets/Characters/MainCharacter/BPs/Blueprints/InvisibleMesh.InvisibleMesh"))) 500.0) (.rotation (`self.MovementY` (`self.MovementSpeedCalc`) (`self.FastMoveMult`) AxisValue "/Game/MainAssets/Characters/MainCharacter/BPs/Blueprints/InvisibleMesh.InvisibleMesh")) (.scale (`self.MovementY` (`self.MovementSpeedCalc`) (`self.FastMoveMult`) AxisValue "/Game/MainAssets/Characters/MainCharacter/BPs/Blueprints/InvisibleMesh.InvisibleMesh"))) false false))

(event `InputAxisKey|MouseX`
  (params (AxisValue :type "Float (single-precision)"))
  (bind _panspeed (`self.PanSpeed`))
  (bind _invisible_mesh (`self.Invisible Mesh`))
  ;[1 1 1] Panning and Edge Scroll
  (bind (_deltaxspeed _deltayspeed) (`self.ScreenEdgeScroll` :!label _label))
  (`self.K2_AddActorLocalOffset` (`KismetMathLibrary.MakeVector` _deltaxspeed _deltayspeed) true)
  (`/Engine/EditorBlueprintResources/StandardMacros.Gate` true :!label _label_2
    (:`Exit`
      (`SceneComponent.K2_SetWorldRotation` _invisible_mesh (`KismetMathLibrary.MakeRotator` (.roll (`SceneComponent.K2_GetComponentRotation` _invisible_mesh)) (`KismetMathLibrary.FClamp` (+ (.pitch (`SceneComponent.K2_GetComponentRotation` _invisible_mesh)) (* _panspeed (stale `InputAxisKey|MouseY` AxisValue))) -80.0 45.0) (+ (.yaw (`SceneComponent.K2_GetComponentRotation` _invisible_mesh)) (* AxisValue _panspeed))) false false))))

(event `Key|LeftShift`
  (params (Key :type "Key Structure"))
  ;[1 1 1] Camera Movement
  (:`Pressed`
    (set `self.FastMoveMult` 5.0))
  (:`Released`
    (set `self.FastMoveMult` 1.0)))

(event `InputAxisKey|MouseY`
  (params (AxisValue :type "Float (single-precision)"))
  ;[1 1 1] Panning and Edge Scroll
  (goto _label :!via `MouseY`))

(event `InputAction|ZoomReset`
  (params (Key :type "Key Structure"))
  ;[1 1 1] Zoom Control
  (:`Pressed`
    (set `SpringArmComponent.TargetArmLength` 1500.0 (`self.SpringArm`))))

(event `InputAction|PanReset`
  (params (Key :type "Key Structure"))
  (bind _camera (`self.Camera`))
  ;[1 1 1] PanReset
  (:`Pressed`
    (`SceneComponent.K2_SetWorldRotation` _camera (`KismetMathLibrary.MakeRotator` (.roll (`SceneComponent.K2_GetComponentRotation` _camera)) 0.0 (.yaw (`SceneComponent.K2_GetComponentRotation` _camera))) false false)))

(event `InputAction|ZoomIn`
  (params (Key :type "Key Structure"))
  (bind _springarm (`self.SpringArm`))
  ;[1 1 1] Zoom Control
  (:`Pressed`
    (set `SpringArmComponent.TargetArmLength` (`KismetMathLibrary.FClamp` (- (`SpringArmComponent.TargetArmLength` _springarm) (`self.ZoomSpeed`)) (`self.MinZoomLimit`) (`self.MaxZoomLimit`)) _springarm)))

(event `InputAction|ZoomOut`
  (params (Key :type "Key Structure"))
  (bind _springarm (`self.SpringArm`))
  ;[1 1 1] Zoom Control
  (:`Pressed`
    (set `SpringArmComponent.TargetArmLength` (`KismetMathLibrary.FClamp` (+ (`self.ZoomSpeed`) (`SpringArmComponent.TargetArmLength` _springarm)) (`self.MinZoomLimit`) (`self.MaxZoomLimit`)) _springarm)))

(event `self.ReceiveTick`
  (params (DeltaSeconds :type "Float (single-precision)"))
  (bind (_hitresult _returnvalue) (`PlayerController.GetHitResultUnderCursorByChannel` (`GameplayStatics.GetPlayerController` 0) "TraceTypeQuery1" true))
  (bind (_bblockinghit _binitialoverlap _time _distance _location) (`GameplayStatics.BreakHitResult` _hitresult))
  ;[1 1 1] Spawn Particle at Mouse Along Floor
  (`/Engine/EditorBlueprintResources/StandardMacros.Gate` true :!label _label_3
    (:`Exit`
      (if _returnvalue
        (`GameplayStatics.SpawnEmitterAtLocation` null (`KismetMathLibrary.MakeVector` (.x _location) (.y _location) (+ (.z _location) 10.0)))))))

(event `Key|LeftMouseButton`
  (params (Key :type "Key Structure"))
  (bind _returnvalue (`GameplayStatics.GetPlayerController` 0))
  ;[1 1 1] Spawn Particle at Mouse Along Floor
  (:`Pressed`
    (set `PlayerController.bShowMouseCursor` false _returnvalue)
    (goto _label_3 :!via `Open`))
  (:`Released`
    (set `PlayerController.bShowMouseCursor` true _returnvalue)
    (goto _label_3 :!via `Close`)))

(fn `MovementSpeedCalc`
  (returns (MovementSensitivity :type "Float (double-precision)"))
  (return (`KismetMathLibrary.FClamp` (/ (`SpringArmComponent.TargetArmLength` (`self.SpringArm`)) 100.0) 5.0 20.0)))

(fn `SetHUDVisibility`
  (params (GameTimeHUD :type "ESlateVisibility Enum" :default "Visible"))
  (`Widget.SetVisibility` (`self.Hud_CNC_Ref`) GameTimeHUD))

(fn `UserConstructionScript`)