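; Player crafting component that builds craft slots from a recipe array through the inventory component's widget and crafts items into that inventory.
; Crafting spawns a BP_MasterPickup by enum to get its item info, then removes ingredients once the inventory accepts it.
; Removal chains up to five requirements, draining the first matching slot.
; Any shortfall re-runs the whole chain from requirement one with only that requirement's amount reduced.
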(event `Init`
  (`/Engine/EditorBlueprintResources/StandardMacros.IsValid` (`self.InventoryComponent`)
    (:`Is Valid`
      (`self.fGenerateCraftSlots`)
      (`self.fUpdateCraftSlots`)
      (set `/Game/MainAssets/Blueprints/Player_BPs/BP_InventoryComponent.CraftingComponent` self (`self.InventoryComponent`)))
    (:`Is Not Valid`
      (`KismetSystemLibrary.PrintString` "Crafting component got fucked and has no ref to the inventory component"))))

(fn `fAddItem`
  (params (ItemInfo :type "/Game/MainAssets/Blueprints/Structures/ItemStruct Structure"))
  (returns (Success :type Boolean))
  (bind _success (`/Game/MainAssets/Blueprints/Player_BPs/BP_InventoryComponent.PickUpItem` (`self.InventoryComponent`) ItemInfo))
  (return _success))

(fn `fCraftItem`
  (params (CraftItemInfo :type "/Game/MainAssets/Blueprints/Structures/CraftRecipes Structure"))
  (locals (L_CraftItemInfo :type "/Game/MainAssets/Blueprints/Structures/CraftRecipes Structure"))
  (bind _output_get (set `local.L_CraftItemInfo` CraftItemInfo))
  (bind _returnvalue (`|SpawnActorFromClass` "/Game/MainAssets/Blueprints/Player_BPs/BP_MasterPickup.BP_MasterPickup_C" (`KismetMathLibrary.MakeTransform` (0.0 0.0 7.766279436516721e+18)) "AdjustIfPossibleButAlwaysSpawn" "OverrideRootScale" null (`.Name_5_2B1B95BE40E628FBA0130FBC97B2CE67` (break `/Game/MainAssets/Blueprints/Structures/CraftRecipes` _output_get)) null))
  (bind _success (`/Game/MainAssets/Blueprints/Player_BPs/BP_InventoryComponent.PickUpItem` (`self.InventoryComponent`) (`/Game/MainAssets/Blueprints/Player_BPs/BP_MasterPickup.ItemInfo` _returnvalue)))
  (if _success
    (`Actor.K2_DestroyActor` _returnvalue)
    (`self.RemoveMultipleItems` (`local.L_CraftItemInfo`))
    (else
      (`KismetSystemLibrary.PrintString` "Fuck \nFailed to add item \nCheck the master BP Pickup \nPossible cause is array element not set"))))

(fn `fGenerateCraftSlots`
  (bind _arrayofrecipes (`self.ArrayOfRecipes`))
  (for _array_element _arrayofrecipes
    (if (`|EnumEquality` (`.CraftType_8_D6BDFE554B16276C19D116A5E3B9EB7D` (break `/Game/MainAssets/Blueprints/Structures/CraftRecipes` _array_element)) (`self.CraftType`))
      _))
  (message `/Game/MainAssets/Blueprints/Player_BPs/BP_InventoryWidgInterface.GenerateCraftSlots` (`/Game/MainAssets/Blueprints/Player_BPs/BP_InventoryComponent.W_Ref` (`self.InventoryComponent`)) _arrayofrecipes self))

(fn `FindItemSlotByNameWithAmount`
  (params (Name :type "/Game/MainAssets/Blueprints/Enums/Enum_ItemType Enum" :default "NewEnumerator14"))
  (returns (ItemInfo :type "/Game/MainAssets/Blueprints/Structures/ItemStruct Structure") (Index :type Integer) (AmountInSlot :type Integer))
  (locals (L_AmountInSlot :type Integer) (L_SlotIndex :type Integer) (L_ItemInfo :type "/Game/MainAssets/Blueprints/Structures/ItemStruct Structure"))
  (for (_array_element _array_index) (`/Game/MainAssets/Blueprints/Player_BPs/BP_InventoryComponent.ArrayOfSlots` (`self.InventoryComponent`))
    (bind ((`Amount_27_FC67A8E34DBED97F84EF428B5041EAB0` _amount) (`EnumType_31_1670885A408965D04ABA14BE39E2FDC7` _enumtype)) (break `/Game/MainAssets/Blueprints/Structures/ItemStruct` _array_element))
    (if (`|EnumEquality` _enumtype Name)
      (set `local.L_AmountInSlot` _amount)
      (set `local.L_SlotIndex` _array_index)
      (set `local.L_ItemInfo` _array_element)
      (break)))
  (return (`local.L_ItemInfo`) (`local.L_SlotIndex`) (`local.L_AmountInSlot`)))

(fn `fUpdateCraftSlots`
  (bind _inventorycomponent (`self.InventoryComponent`))
  (message `/Game/MainAssets/Blueprints/Player_BPs/BP_InventoryWidgInterface.UpdateCraftSlots` (`/Game/MainAssets/Blueprints/Player_BPs/BP_InventoryComponent.W_Ref` _inventorycomponent) (`self.ArrayOfRecipes`) _inventorycomponent))

(fn `GetAmountOfItemsByEnum`
  (params (InventorySlotToSearch :type "/Game/MainAssets/Blueprints/Player_BPs/BP_InventoryComponent Object Reference") (Name :type "/Game/MainAssets/Blueprints/Enums/Enum_ItemType Enum" :default "NewEnumerator14"))
  (returns (L_Amount1 :type Integer))
  (locals (L_Amount :type Integer))
  (set `local.L_Amount` 0)
  (for _array_element (`/Game/MainAssets/Blueprints/Player_BPs/BP_InventoryComponent.ArrayOfSlots` InventorySlotToSearch)
    (bind ((`Amount_27_FC67A8E34DBED97F84EF428B5041EAB0` _amount) (`EnumType_31_1670885A408965D04ABA14BE39E2FDC7` _enumtype)) (break `/Game/MainAssets/Blueprints/Structures/ItemStruct` _array_element))
    (if (`|EnumEquality` _enumtype Name)
      (set `local.L_Amount` (+ (`local.L_Amount`) _amount))))
  (return (`local.L_Amount`)))

(fn `RemoveMultipleItems`
  (params (CraftItemInfo :type "/Game/MainAssets/Blueprints/Structures/CraftRecipes Structure"))
  (locals (L_CraftRecipe :type "/Game/MainAssets/Blueprints/Structures/CraftRecipes Structure") (L_RemainingAmountToMove :type Integer :default 0))
  (bind _inventorycomponent (`self.InventoryComponent`))
  (bind _inventorycomponent_2 (`self.InventoryComponent`))
  (bind _inventorycomponent_3 (`self.InventoryComponent`))
  (bind _inventorycomponent_4 (`self.InventoryComponent`))
  (bind _inventorycomponent_5 (`self.InventoryComponent`))
  (bind (_icon _name _crafttype _requirement1 _requirement1amount _requirement2 _requirement2amount _requirement3 _requirement3amount _requirement4 _requirement4amount _requirement5) (break `/Game/MainAssets/Blueprints/Structures/CraftRecipes` (`local.L_CraftRecipe`)))
  (bind (_icon_2 _name_2 _crafttype_2 _requirement1_2 _requirement1amount_2 _requirement2_2 _requirement2amount_2 _requirement3_2 _requirement3amount_2 _requirement4_2 _requirement4amount_2 _requirement5_2 _requirement5amount) (break `/Game/MainAssets/Blueprints/Structures/CraftRecipes` (`local.L_CraftRecipe`)))
  (bind (_icon_3 _name_3 _crafttype_3 _requirement1_3 _requirement1amount_3 _requirement2_3 _requirement2amount_3 _requirement3_3 _requirement3amount_3 _requirement4_3 _requirement4amount_3 _requirement5_3 _requirement5amount_2) (break `/Game/MainAssets/Blueprints/Structures/CraftRecipes` (`local.L_CraftRecipe`)))
  (bind (_icon_4 _name_4 _crafttype_4 _requirement1_4 _requirement1amount_4 _requirement2_4 _requirement2amount_4 _requirement3_4 _requirement3amount_4 _requirement4_4 _requirement4amount_4 _requirement5_4 _requirement5amount_3) (break `/Game/MainAssets/Blueprints/Structures/CraftRecipes` (`local.L_CraftRecipe`)))
  (bind (_icon_5 _name_5 _crafttype_5 _requirement1_5 _requirement1amount_5 _requirement2_5 _requirement2amount_5 _requirement3_5 _requirement3amount_5 _requirement4_5 _requirement4amount_5 _requirement5_5 _requirement5amount_4) (break `/Game/MainAssets/Blueprints/Structures/CraftRecipes` (`local.L_CraftRecipe`)))
  (bind _output_get (set `local.L_CraftRecipe` CraftItemInfo))
  (bind (_icon_6 _name_6 _crafttype_6 _requirement1_6 _requirement1amount_6 _requirement2_6 _requirement2amount_6 _requirement3_6 _requirement3amount_6 _requirement4_6 _requirement4amount_6 _requirement5_6 _requirement5amount_5) (break `/Game/MainAssets/Blueprints/Structures/CraftRecipes` _output_get))
  (bind (_iteminfo _index _amountinslot) (`self.FindItemSlotByNameWithAmount` _requirement1_6))
  (if (> _amountinslot _requirement1amount_6)
    (`/Game/MainAssets/Blueprints/Player_BPs/BP_InventoryComponent.RemoveAmountFromSlot` _inventorycomponent_2 _iteminfo _index _requirement1amount_6)
    (`self.fUpdateCraftSlots`)
    (if (`|EnumEquality` _requirement2_6 "NewEnumerator14") :!label _label
      (`self.fUpdateCraftSlots`)
      (else
        (bind (_iteminfo_2 _index_2 _amountinslot_2) (`self.FindItemSlotByNameWithAmount` _requirement2_6))
        (if (> _amountinslot_2 _requirement2amount_6)
          (`/Game/MainAssets/Blueprints/Player_BPs/BP_InventoryComponent.RemoveAmountFromSlot` _inventorycomponent_3 _iteminfo_2 _index_2 _requirement2amount_6)
          (`self.fUpdateCraftSlots`)
          (if (`|EnumEquality` _requirement3_6 "NewEnumerator14") :!label _label_2
            (`self.fUpdateCraftSlots`)
            (else
              (bind (_iteminfo_3 _index_3 _amountinslot_3) (`self.FindItemSlotByNameWithAmount` _requirement3_6))
              (if (> _amountinslot_3 _requirement3amount_6)
                (`/Game/MainAssets/Blueprints/Player_BPs/BP_InventoryComponent.RemoveAmountFromSlot` _inventorycomponent_4 _iteminfo_3 _index_3 _requirement3amount_6)
                (`self.fUpdateCraftSlots`)
                (if (`|EnumEquality` _requirement4_6 "NewEnumerator14") :!label _label_3
                  (`self.fUpdateCraftSlots`)
                  (else
                    (bind (_iteminfo_4 _index_4 _amountinslot_4) (`self.FindItemSlotByNameWithAmount` _requirement4_6))
                    (if (> _amountinslot_4 _requirement4amount_6)
                      (`/Game/MainAssets/Blueprints/Player_BPs/BP_InventoryComponent.RemoveAmountFromSlot` _inventorycomponent_5 _iteminfo_4 _index_4 _requirement4amount_6)
                      (`self.fUpdateCraftSlots`)
                      (if (`|EnumEquality` _requirement5_6 "NewEnumerator14") :!label _label_4
                        (`self.fUpdateCraftSlots`)
                        (else
                          (bind (_iteminfo_5 _index_5 _amountinslot_5) (`self.FindItemSlotByNameWithAmount` _requirement5_6))
                          (if (> _amountinslot_5 _requirement5amount_5)
                            (`/Game/MainAssets/Blueprints/Player_BPs/BP_InventoryComponent.RemoveAmountFromSlot` _inventorycomponent _iteminfo_5 _index_5 _requirement5amount_5)
                            (`self.fUpdateCraftSlots`)
                            (else
                              (`/Game/MainAssets/Blueprints/Player_BPs/BP_InventoryComponent.Remove Item from Slot` _inventorycomponent _index_5)
                              (bind _returnvalue (- _requirement5amount_5 _amountinslot_5))
                              (if (not (== _returnvalue 0))
                                (set `local.L_RemainingAmountToMove` _returnvalue)
                                (`self.RemoveMultipleItems` (make `/Game/MainAssets/Blueprints/Structures/CraftRecipes` _icon _name _crafttype _requirement1 _requirement1amount _requirement2 _requirement2amount _requirement3 _requirement3amount _requirement4 _requirement4amount _requirement5 (`local.L_RemainingAmountToMove`))))))))
                      (else
                        (`/Game/MainAssets/Blueprints/Player_BPs/BP_InventoryComponent.Remove Item from Slot` _inventorycomponent_5 _index_4)
                        (bind _returnvalue_2 (- _requirement4amount_6 _amountinslot_4))
                        (if (== _returnvalue_2 0)
                          (goto _label_4)
                          (else
                            (set `local.L_RemainingAmountToMove` _returnvalue_2)
                            (`self.RemoveMultipleItems` (make `/Game/MainAssets/Blueprints/Structures/CraftRecipes` _icon_5 _name_5 _crafttype_5 _requirement1_5 _requirement1amount_5 _requirement2_5 _requirement2amount_5 _requirement3_5 _requirement3amount_5 _requirement4_5 (`local.L_RemainingAmountToMove`) _requirement5_5 _requirement5amount_4))))))))
                (else
                  (`/Game/MainAssets/Blueprints/Player_BPs/BP_InventoryComponent.Remove Item from Slot` _inventorycomponent_4 _index_3)
                  (bind _returnvalue_3 (- _requirement3amount_6 _amountinslot_3))
                  (if (== _returnvalue_3 0)
                    (goto _label_3)
                    (else
                      (set `local.L_RemainingAmountToMove` _returnvalue_3)
                      (`self.RemoveMultipleItems` (make `/Game/MainAssets/Blueprints/Structures/CraftRecipes` _icon_4 _name_4 _crafttype_4 _requirement1_4 _requirement1amount_4 _requirement2_4 _requirement2amount_4 _requirement3_4 (`local.L_RemainingAmountToMove`) _requirement4_4 _requirement4amount_4 _requirement5_4 _requirement5amount_3))))))))
          (else
            (`/Game/MainAssets/Blueprints/Player_BPs/BP_InventoryComponent.Remove Item from Slot` _inventorycomponent_3 _index_2)
            (bind _returnvalue_4 (- _requirement2amount_6 _amountinslot_2))
            (if (== _returnvalue_4 0)
              (goto _label_2)
              (else
                (set `local.L_RemainingAmountToMove` _returnvalue_4)
                (`self.RemoveMultipleItems` (make `/Game/MainAssets/Blueprints/Structures/CraftRecipes` _icon_3 _name_3 _crafttype_3 _requirement1_3 _requirement1amount_3 _requirement2_3 (`local.L_RemainingAmountToMove`) _requirement3_3 _requirement3amount_3 _requirement4_3 _requirement4amount_3 _requirement5_3 _requirement5amount_2))))))))
    (else
      (`/Game/MainAssets/Blueprints/Player_BPs/BP_InventoryComponent.Remove Item from Slot` _inventorycomponent_2 _index)
      (bind _returnvalue_5 (- _requirement1amount_6 _amountinslot))
      (if (== _returnvalue_5 0)
        (goto _label)
        (else
          (set `local.L_RemainingAmountToMove` _returnvalue_5)
          (`self.RemoveMultipleItems` (make `/Game/MainAssets/Blueprints/Structures/CraftRecipes` _icon_2 _name_2 _crafttype_2 _requirement1_2 (`local.L_RemainingAmountToMove`) _requirement2_2 _requirement2amount_2 _requirement3_2 _requirement3amount_2 _requirement4_2 _requirement4amount_2 _requirement5_2 _requirement5amount)))))))