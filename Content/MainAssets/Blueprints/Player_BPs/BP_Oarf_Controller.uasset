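; Player controller for the Oarf character, handling item pickup, storage, inventory and crafting, pawn switching and base building.
; BeginPlay creates the inventory HUD and links it to the inventory and crafting components.
; Building previews follow a camera trace every Tick, snapping floors and walls using the hit point in the target piece's local space.
; Camera switching spawns and possesses an RTS or Oarf pawn; zoom and RTS HUD logic are unwired.
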(event `InputAction|Interact`
  (params (Key :type "Key Structure"))
  (bind _as_bp_oarf (`self.As BP Oarf`))
  (bind _currentlookingatpickupitem (`/Game/MainAssets/Blueprints/Player_BPs/BP_Oarf.CurrentLookingAtPickUpItem` _as_bp_oarf))
  (bind _currentlookatstorage (`/Game/MainAssets/Blueprints/Player_BPs/BP_Oarf.CurrentLookAtStorage` _as_bp_oarf))
  (bind _craftingcomponent (`/Game/MainAssets/Blueprints/Player_BPs/BP_MasterStructure.CraftingComponent` _currentlookatstorage))
  (bind _inventorycomponent (`/Game/MainAssets/Blueprints/Player_BPs/BP_MasterStructure.InventoryComponent` _currentlookatstorage))
  ;[1 1 1] Pick up Item with interact, or "E" and add to inventory
  (:`Pressed`
    (if (`/Game/MainAssets/Blueprints/Player_BPs/BP_Oarf.CanPickUpItem` _as_bp_oarf)
      (bind _success (`/Game/MainAssets/Blueprints/Player_BPs/BP_InventoryComponent.PickUpItem` (`self.InventoryComponent`) (`/Game/MainAssets/Blueprints/Player_BPs/BP_MasterPickup.ItemInfo` _currentlookingatpickupitem)))
      (if _success
        (`self.K2_DestroyActor` _currentlookingatpickupitem))
      (elif (`/Game/MainAssets/Blueprints/Player_BPs/BP_Oarf.CanOpenStorage` _as_bp_oarf)
        (if (not (`/Game/MainAssets/Blueprints/Player_BPs/BP_InventoryComponent.bIsInventoryOpen` _inventorycomponent))
          (`/Game/MainAssets/Blueprints/Player_BPs/BP_InventoryComponent.OpenCloseInventory` (`self.InventoryComponent`))
          (`/Game/MainAssets/Blueprints/Player_BPs/BP_InventoryComponent.OpenCloseInventory` _inventorycomponent)
          (set `self.SecondInventory` _inventorycomponent)
          (`/Engine/EditorBlueprintResources/StandardMacros.IsValid` _craftingcomponent
            (:`Is Valid`
              (`/Game/MainAssets/Blueprints/Player_BPs/CraftingComponent.fUpdateCraftSlots` _craftingcomponent))))))))

(event `self.ReceiveBeginPlay`
  (bind _craftingcomponent (`self.CraftingComponent`))
  (bind _inventorycomponent (`self.InventoryComponent`))
  ;[1 1 1] Begin Play for creating HUD widget
  (bind _asbp_oarf (cast `/Game/MainAssets/Blueprints/Player_BPs/BP_Oarf` (`self.K2_GetPawn`)))
  (set `self.As BP Oarf` _asbp_oarf)
  (bind _returnvalue (`|CreateWidget` "/Game/MainAssets/Blueprints/Widgets/Widg_HUD_Inv.Widg_HUD_Inv_C" self))
  (bind _output_get (set `self.HUD` _returnvalue))
  (`UserWidget.AddToViewport` _output_get 0)
  (`ActorComponent.Activate` _inventorycomponent false)
  (set `/Game/MainAssets/Blueprints/Player_BPs/BP_InventoryComponent.W_HUD` (`self.HUD`) _inventorycomponent)
  (`/Engine/EditorBlueprintResources/StandardMacros.IsValid` _craftingcomponent
    (:`Is Valid`
      (set `/Game/MainAssets/Blueprints/Player_BPs/CraftingComponent.InventoryComponent` (`self.InventoryComponent`) _craftingcomponent)
      (`/Game/MainAssets/Blueprints/Player_BPs/CraftingComponent.Init` _craftingcomponent))))

(event `InputAction|Alt Down`
  (params (Key :type "Key Structure"))
  ;[1 1 1] Your standard input actions for shift and alt
  (:`Pressed`
    (set `self.bAltDown` true))
  (:`Released`
    (set `self.bAltDown` false)))

(event `InputAction|OpenInventory`
  (params (Key :type "Key Structure"))
  ;[1 1 1] Open inventory by pressing "Tab" or "i"
  (:`Pressed`
    (`/Game/MainAssets/Blueprints/Player_BPs/BP_InventoryComponent.OpenCloseInventory` (`self.InventoryComponent`))
    (`/Game/MainAssets/Blueprints/Player_BPs/CraftingComponent.fUpdateCraftSlots` (`self.CraftingComponent`))
    (`self.CheckToCloseOtherInventories`)))

(event `self.InventoryComponent.OnComponentActivated`
  (params (Component :type "ActorComponent Object Reference") (bReset :type Boolean))
  ;[1 1 1] Create HUD upon activating
  (bind _asbp_inventory_component (cast `/Game/MainAssets/Blueprints/Player_BPs/BP_InventoryComponent` Component))
  (set `/Game/MainAssets/Blueprints/Player_BPs/BP_InventoryComponent.W_HUD` (`self.HUD`) _asbp_inventory_component)
  (`/Game/MainAssets/Blueprints/Player_BPs/BP_InventoryComponent.Init` _asbp_inventory_component))

(event `InputAction|Shift Down`
  (params (Key :type "Key Structure"))
  ;[1 1 1] Your standard input actions for shift and alt
  (:`Pressed`
    (set `self.bShiftDown` true))
  (:`Released`
    (set `self.bShiftDown` false)))

(event `InputAction|SwitchCameraPawn`
  (params (Key :type "Key Structure"))
  (bind _returnvalue (`GameplayStatics.GetPlayerController` 0))
  (bind _returnvalue_2 (`GameplayStatics.GetPlayerController` 0))
  ;[1 1 1] Switch Camera Pawn
  (:`Pressed`
    (`/Engine/EditorBlueprintResources/StandardMacros.FlipFlop`
      (:`A`
        (`self.UnPossess` _returnvalue)
        (bind _returnvalue_3 (`|SpawnActorFromClass` "/Game/MainAssets/Blueprints/Player_BPs/BP_RTSCameraPawn.BP_RTSCameraPawn_C" (`self.GetTransform` _returnvalue) "Undefined" "OverrideRootScale" null null))
        (`self.K2_TeleportTo` _returnvalue_3 (`self.K2_GetActorLocation` (stale _returnvalue_4)) (`self.K2_GetActorRotation` (stale _returnvalue_4)))
        (`self.Possess` _returnvalue _returnvalue_3)
        (`self.K2_DestroyActor` (stale _returnvalue_4))
        (`self.K2_DestroyActor` _returnvalue)
        (set `self.bShowMouseCursor` true))
      (:`B`
        (`self.UnPossess` _returnvalue_2)
        (bind _returnvalue_4 (`|SpawnActorFromClass` "/Game/MainAssets/Blueprints/Player_BPs/BP_Oarf.BP_Oarf_C" (`self.GetTransform` _returnvalue_2) "Undefined" "OverrideRootScale" null null))
        (`self.K2_TeleportTo` _returnvalue_4 (`self.K2_GetActorLocation` _returnvalue_3) (`KismetMathLibrary.MakeRotator` (.roll (`self.K2_GetActorRotation` _returnvalue_3))))
        (`self.Possess` _returnvalue_2 _returnvalue_4)
        (`self.K2_DestroyActor` _returnvalue_3)
        (`self.K2_DestroyActor` (`self.CameraPawnRef`))
        (set `self.bShowMouseCursor` false)))))

(event `InputAction|ZoomReset`
  (params (Key :type "Key Structure"))
  ;[1 1 1] Zoom Function
)

(event `InputAction|Toggle_Build_Floor`
  (params (Key :type "Key Structure"))
  ;[1 1 1] ToggleBuild
  (:`Pressed`
    (set `self.BuildClass` "/Game/MainAssets/Buildings/BPs/BP_Building_Floor.BP_Building_Floor_C")
    (if (`self.IsBuilding`) :!label _label
      (set `self.IsBuilding` false)
      (`self.K2_DestroyActor` (`self.Building`))
      (`self.PositionBuild`)
      (else
        (set `self.IsBuilding` true)
        (`self.SpawnBuildItem`)))))

(event `InputAction|Toggle_Build_Wall`
  (params (Key :type "Key Structure"))
  ;[1 1 1] ToggleBuild
  (:`Pressed`
    (set `self.BuildClass` "/Game/MainAssets/Buildings/BPs/BP_Building_Wall.BP_Building_Wall_C")
    (goto _label)))

(event `InputAction|ZoomIn`
  (params (Key :type "Key Structure"))
  ;[1 1 1] Zoom Function
)

(event `InputAction|ZoomOut`
  (params (Key :type "Key Structure"))
  ;[1 1 1] Zoom Function
)

(event `self.ReceiveTick`
  (params (DeltaSeconds :type "Float (single-precision)"))
  ;[1 1 1] SpawnActualBuilding
  (if (`self.IsBuilding`)
    (`self.PositionBuild`)
    (if (`self.ClickedToPlace`)
      (set `self.ClickedToPlace` false)
      (`PrimitiveComponent.SetCollisionEnabled` (`/Game/MainAssets/Buildings/BPs/BP_Building_Base.Mesh` (`self.Building`)) "QueryAndPhysics")
      (`self.SpawnBuildItem`))))

(event `InputAction|PlaceBuilding`
  (params (Key :type "Key Structure"))
  ;[1 1 1] PlaceBuilding
  (:`Pressed`
    (if (`self.IsBuilding`)
      (set `self.ClickedToPlace` true))))

(event `InputAction|RotateBuilding`
  (params (Key :type "Key Structure"))
  ;[1 1 1] RotateBuilding
  (:`Pressed`
    (set `self.ShouldRotate` true))
  (:`Released`
    (set `self.ShouldRotate` false)))

(event `InputAction|CycleBuilding`
  (params (Key :type "Key Structure"))
  ;[1 1 1] CycleBuilding
  (:`Pressed`
    (if (`self.IsBuilding`)
      (`/Game/MainAssets/Buildings/BPs/BP_Building_Base.NextMesh` (`self.Building`)))))

(event `InputAction|DeleteBuilding`
  (params (Key :type "Key Structure"))
  ;[1 1 1] Fuck that shit up
  (:`Pressed`
    (bind (_bblockinghit _impactpoint _hititem) (`self.CameraTrace`))
    (`/Engine/EditorBlueprintResources/StandardMacros.IsValid` _hititem
      (:`Is Valid`
        (`self.K2_DestroyActor` _hititem)))))

(fn `CameraTrace`
  (returns (bBlockingHit :type Boolean) (ImpactPoint :type "Vector Structure") (HitItem :type "/Game/MainAssets/Buildings/BPs/BP_Building_Base Object Reference") (HitBuildItem :type Boolean))
  (bind _asbp_oarf (cast `/Game/MainAssets/Blueprints/Player_BPs/BP_Oarf` (`GameplayStatics.GetPlayerCharacter` 0))
    (:`then`
      (bind _camera (`/Game/MainAssets/Blueprints/Player_BPs/BP_Oarf.Camera` _asbp_oarf))
      (bind _returnvalue (`SceneComponent.K2_GetComponentLocation` _camera))
      (bind _outhit (`KismetSystemLibrary.LineTraceSingleForObjects` :`Start` _returnvalue :`End` (+ _returnvalue (* (`SceneComponent.GetForwardVector` _camera) 20000.0)) :`ObjectTypes` (`|MakeArray` "ObjectTypeQuery7" :!type "EObjectTypeQuery Enum") :`DrawDebugType` "ForDuration")))
    (:`CastFailed`
      _))
  (bind (_bblockinghit _binitialoverlap _time _distance _location _impactpoint _normal _impactnormal _physmat _hitactor) (`GameplayStatics.BreakHitResult` _outhit))
  (bind (_asbp_building_base _bsuccess) (cast `/Game/MainAssets/Buildings/BPs/BP_Building_Base` _hitactor :!pure true))
  (return _bblockinghit _impactpoint _asbp_building_base _bsuccess))

(fn `CheckToCloseOtherInventories`
  (bind _secondinventory (`self.SecondInventory`))
  (`/Engine/EditorBlueprintResources/StandardMacros.IsValid` _secondinventory
    (:`Is Valid`
      (`/Game/MainAssets/Blueprints/Player_BPs/BP_InventoryComponent.OpenCloseInventory` _secondinventory)
      (set `self.SecondInventory` null))))

(fn `PositionBuild`
  (locals (Hit :type "Vector Structure" :default (0.0 0.0 0.0)) (HitItem :type "/Game/MainAssets/Buildings/BPs/BP_Building_Base Object Reference") (XOffset :type "Float (double-precision)") (YOffset :type "Float (double-precision)") (OffsetAmount :type "Float (double-precision)") (NeedRotate :type Boolean) (WallSnap :type Boolean))
  (bind _building (`self.Building`))
  (bind (_bblockinghit _impactpoint _hititem _hitbuilditem) (`self.CameraTrace`))
  (set `local.HitItem` _hititem)
  (set `local.Hit` _impactpoint)
  (if _bblockinghit
    (if _hitbuilditem
      (switch `string` (`KismetSystemLibrary.GetClassDisplayName` (`GameplayStatics.GetObjectClass` (`self.Building`)))
        (:`BP_Building_Wall_C`
          (switch `string` (`KismetSystemLibrary.GetClassDisplayName` (`GameplayStatics.GetObjectClass` (`local.HitItem`)))
            (:`BP_Building_Wall_C`
              (`self.SnapWallToWall` (`local.HitItem`) (`local.Hit`)))
            (:`BP_Building_Floor_C`
              (`self.SnapToFloor` true (`local.HitItem`) (`local.Hit`)))))
        (:`BP_Building_Floor_C`
          (switch `string` (`KismetSystemLibrary.GetClassDisplayName` (`GameplayStatics.GetObjectClass` (`local.HitItem`)))
            (:`BP_Building_Wall_C`
              (`self.SnapFloorToWall` (`local.HitItem`) (`local.Hit`)))
            (:`BP_Building_Floor_C`
              (`self.SnapToFloor` false (`local.HitItem`) (`local.Hit`))))))
      (else
        (`/Engine/EditorBlueprintResources/StandardMacros.IsValid` _building
          (:`Is Valid`
            (`self.K2_SetActorLocation` _building _impactpoint false false)
            (if (`self.ShouldRotate`)
              (`self.K2_AddActorWorldRotation` _building (struct :`Yaw` 0.5) false false)))
          (:`Is Not Valid`
            (`self.K2_DestroyActor`)))))))

(fn `SetBuildSize`)

(fn `SetHUD_Visibility`
  (params (InVisibility :type "ESlateVisibility Enum" :default "Visible"))
  (`Widget.SetVisibility` (`self.Hud_CNC_Ref`) InVisibility))

(fn `SnapFloorToWall`
  (params (SnapTo :type "Actor Object Reference") (Hit :type "Vector Structure"))
  (locals (ZOffset :type "Float (double-precision)") (YOffset :type "Float (double-precision)"))
  (bind _returnvalue (`self.GetTransform` SnapTo))
  (bind _building (`self.Building`))
  (bind (_returnvalue_x _returnvalue_y _returnvalue_z) (`KismetMathLibrary.BreakVector` (`KismetMathLibrary.InverseTransformLocation` _returnvalue Hit)))
  (bind (_returnvalue_roll _returnvalue_pitch _returnvalue_yaw) (`KismetMathLibrary.BreakRotator` (`KismetMathLibrary.NormalizedDeltaRotator` (`KismetMathLibrary.Conv_VectorToRotator` (`self.GetActorRightVector` SnapTo)) (`KismetMathLibrary.Conv_VectorToRotator` (- (`self.K2_GetActorLocation` (`GameplayStatics.GetPlayerPawn` 0)) (`self.K2_GetActorLocation` SnapTo))))))
  (if (> _returnvalue_z 200.0)
    (set `local.ZOffset` 400.0))
  (if (> (`KismetMathLibrary.Abs` _returnvalue_yaw) 90.0)
    (set `local.YOffset` -200.0))
  (`/Engine/EditorBlueprintResources/StandardMacros.IsValid` _building
    (:`Is Valid`
      (`self.K2_SetActorTransform` _building _returnvalue false false)
      (`self.K2_AddActorLocalOffset` _building (`KismetMathLibrary.MakeVector` 0.0 (`local.YOffset`) (`local.ZOffset`)) false false))
    (:`Is Not Valid`
      (`self.K2_DestroyActor`))))

(fn `SnapToFloor`
  (params (PlacingWall :type Boolean) (SnapTo :type "Actor Object Reference") (Hit :type "Vector Structure"))
  (locals (OffsetAmount :type "Float (double-precision)") (YOffset :type "Float (double-precision)") (XOffset :type "Float (double-precision)") (WallSnap :type Boolean) (NeedRotate :type Boolean))
  (bind _building (`self.Building`))
  (bind _offsetamount (`local.OffsetAmount`))
  (bind (_returnvalue_x _returnvalue_y) (`KismetMathLibrary.BreakVector` (`KismetMathLibrary.InverseTransformLocation` (`self.GetTransform` SnapTo) Hit)))
  (bind _output_get (set `local.WallSnap` PlacingWall))
  (if _output_get
    (set `local.OffsetAmount` 200.0)
    (else
      (set `local.OffsetAmount` 400.0)))
  (`/Engine/EditorBlueprintResources/StandardMacros.CompareFloat` (`KismetMathLibrary.Abs` _returnvalue_x) (`KismetMathLibrary.Abs` _returnvalue_y)
    (:`>`
      (set `local.XOffset` (* (`KismetMathLibrary.SignOfFloat` _returnvalue_x) _offsetamount))
      (set `local.NeedRotate` true))
    (:`==`
      (set `local.YOffset` (* (`KismetMathLibrary.SignOfFloat` _returnvalue_y) _offsetamount) :!label _label))
    (:`<`
      (goto _label)))
  (`/Engine/EditorBlueprintResources/StandardMacros.IsValid` _building
    (:`Is Valid`
      (`self.K2_SetActorTransform` _building (`self.GetTransform` SnapTo) false false)
      (`self.K2_AddActorLocalOffset` _building (`KismetMathLibrary.MakeVector` (`local.XOffset`) (`local.YOffset`)) false false)
      (if (and (`local.WallSnap`) (`local.NeedRotate`))
        (`self.K2_AddActorLocalRotation` _building (struct :`Yaw` 90.0) false false)))
    (:`Is Not Valid`
      (`self.K2_DestroyActor`))))

(fn `SnapWallToWall`
  (params (SnapTo :type "Actor Object Reference") (Hit :type "Vector Structure"))
  (locals (XOffset :type "Float (double-precision)") (ZOffset :type "Float (double-precision)"))
  (bind _returnvalue (`self.GetTransform` SnapTo))
  (bind _building (`self.Building`))
  (bind (_returnvalue_x _returnvalue_y _returnvalue_z) (`KismetMathLibrary.BreakVector` (`KismetMathLibrary.InverseTransformLocation` _returnvalue Hit)))
  (`/Engine/EditorBlueprintResources/StandardMacros.CompareFloat` (`KismetMathLibrary.Abs` _returnvalue_x) (`KismetMathLibrary.Abs` (- _returnvalue_z 200.0))
    (:`>`
      (set `local.XOffset` (* (`KismetMathLibrary.SignOfFloat` _returnvalue_x) 400.0))
      (`/Engine/EditorBlueprintResources/StandardMacros.IsValid` _building
        (:`Is Valid`
          (`self.K2_SetActorTransform` _building _returnvalue false false :!label _label)
          (`/Engine/EditorBlueprintResources/StandardMacros.IsValid` _building
            (:`Is Valid`
              (`self.K2_AddActorLocalOffset` _building (`KismetMathLibrary.MakeVector` (`local.XOffset`) 0.0 (`local.ZOffset`)) false false))
            (:`Is Not Valid`
              (`self.K2_DestroyActor` :!label _label_2))))
        (:`Is Not Valid`
          (goto _label_2))))
    (:`==`
      (set `local.ZOffset` (* (`KismetMathLibrary.SignOfFloat` _returnvalue_z) 400.0) :!label _label_3)
      (goto _label))
    (:`<`
      (goto _label_3))))

(fn `SpawnBuildItem`
  (bind _returnvalue (`|SpawnActorFromClass` (`self.BuildClass`) (`KismetMathLibrary.MakeTransform` (0.0 0.0 0.0)) "AlwaysSpawn" "OverrideRootScale" null null))
  (bind _output_get (set `self.Building` _returnvalue))
  (`PrimitiveComponent.SetCollisionEnabled` (`/Game/MainAssets/Buildings/BPs/BP_Building_Base.Mesh` _output_get) "NoCollision"))

(fn `ToggleBuildingNewPart`
  (if (`self.IsBuilding`)
    (`|ExecutionSequence`
      (:`then_0`
        (set `self.IsBuilding` false))
      (:`then_1`
        _))
    (`self.K2_DestroyActor` (`self.Building`))
    (else
      (set `self.IsBuilding` true)
      (`self.SpawnBuildItem`))))

(fn `UserConstructionScript`)