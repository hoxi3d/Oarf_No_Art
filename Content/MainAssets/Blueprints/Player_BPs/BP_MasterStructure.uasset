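; BP_MasterStructure is a structure actor that, through flags, can gain an inventory, crafting and random starting loot.
; On BeginPlay it adds the inventory component, then feeds it into a crafting component built from the recipe list.
; Random loot spawns temporary BP_MasterPickup actors far away from a set of items, copies each into the inventory and destroys it.
; Crafting and loot both require the inventory, and print errors naming the misconfigured actor otherwise.
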(event `self.ReceiveBeginPlay`
  (if (`self.AddInventory`)
    (bind _returnvalue (`AddComponent|NODE_AddBP_InventoryComponent-3` :`bLimitSlots` (`self.LimitSlots`) :`AmountOfSlots` (`self.AmountOfSlots`) :`bShowToolTips` true :`Slot Type` (`self.SlotType`) :`W_Class` (`self.W Class`)))
    (set `self.InventoryComponent` _returnvalue))
  (if (`self.AddCrafting`)
    (if (`self.AddInventory`)
      (bind _returnvalue_2 (`AddComponent|NODE_AddCraftingComponent-0` :`InventoryComponent` (`self.InventoryComponent`) :`ArrayOfRecipes` (`self.ArrayOfRecipes`) :`CraftType` (`self.CraftType`)))
      (bind _output_get (set `self.CraftingComponent` _returnvalue_2))
      (`/Game/MainAssets/Blueprints/Player_BPs/BP_CraftingComponent.Init` _output_get)
      (if (`self.SpawnRandomLoot`) :!label _label
        (if (`self.AddInventory`)
          (for _ (range (`KismetMathLibrary.RandomIntegerInRange` 1 (`self.AmountOfLootItemsToSpawn`)))
            (bind _result (`BlueprintSetLibrary.Set_ToArray` (`self.SetOfItems`)))
            (bind _returnvalue_3 (`|SpawnActorFromClass` "/Game/MainAssets/Blueprints/Player_BPs/BP_MasterPickup.BP_MasterPickup_C" (`KismetMathLibrary.MakeTransform` (0.0 0.0 1.0000000272564224e+16)) "Undefined" "OverrideRootScale" null (`KismetArrayLibrary.Array_Random` _result) null))
            (bind _success (`/Game/MainAssets/Blueprints/Player_BPs/BP_InventoryComponent.PickUpItem` (`self.InventoryComponent`) (`/Game/MainAssets/Blueprints/Player_BPs/BP_MasterPickup.ItemInfo` _returnvalue_3)))
            (if _success
              (`self.K2_DestroyActor` _returnvalue_3)
              (else
                (`KismetSystemLibrary.PrintString` "Failed to add loot check bp_masterstructure" true true (struct :`G` 0.66 :`B` 1.0 :`A` 1.0) 1000.0))))
          (else
            (`KismetSystemLibrary.PrintString` (`KismetStringLibrary.Concat_StrStr` "Error:" "Can't add random loot without inventory" "Solution:" "Please tick \"Add inventory\" checkbox in details panel" "Actor with fault:" (`KismetSystemLibrary.GetDisplayName` self)) true true (struct :`G` 0.66 :`B` 1.0 :`A` 1.0) 1000.0))))
      (else
        (`KismetSystemLibrary.PrintString` (`KismetStringLibrary.Concat_StrStr` "Error:" "Can't add crafting wihtout inventory" "Solution:" "Please tick \"Add inventory\" checkbox in details panel" "Actor with fault:" (`KismetSystemLibrary.GetDisplayName` self)) true true (struct :`G` 0.66 :`B` 1.0 :`A` 1.0) 1000.0)))
    (else
      (goto _label))))

(fn `UserConstructionScript`)