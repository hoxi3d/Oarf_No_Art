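; Storage inventory component that holds item structs in a slot array, optionally pre-filled to a fixed count, and shows them in a storage widget.
; Opening the widget rebuilds its slots and switches cursor and input mode.
; Functions add, stack, split, swap and merge items by editing the array, mostly refreshing the slot widgets afterwards.
; Dropping a slot spawns one BP_MasterPickup per unit ahead of the player at randomised height.
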(event `Init`
  (`self.InventorySetup`)
  (bind _returnvalue (`|CreateWidget` "/Game/MainAssets/Blueprints/Widgets/Widget_Storage.Widget_Storage_C" (`GameplayStatics.GetPlayerController` 0)))
  (set `self.W_StorageRef` _returnvalue))

(fn `AddAmountToItem`
  (params (ItemInfo :type "/Game/MainAssets/Blueprints/Structures/ItemStruct Structure") (SlotIndex :type Integer) (AmountToAdd :type Integer))
  (bind (_name _icon _weight _amount _edibleusable _doesexpire _maxstack _doesstack _emptyslot _description _healthofitem _enumtype) (break `/Game/MainAssets/Blueprints/Structures/ItemStruct` ItemInfo))
  (bind _arrayofslots (`self.ArrayOfSlots`))
  (`KismetArrayLibrary.Array_Set` _arrayofslots SlotIndex (make `/Game/MainAssets/Blueprints/Structures/ItemStruct` _name _icon _weight (+ (`.Amount_27_FC67A8E34DBED97F84EF428B5041EAB0` (break `/Game/MainAssets/Blueprints/Structures/ItemStruct` (`|GetArrayItem` _arrayofslots SlotIndex))) AmountToAdd) _edibleusable _doesexpire _maxstack _doesstack _emptyslot _description _healthofitem _enumtype))
  (return))

(fn `AddItemToArray`
  (params (NewItem :type "/Game/MainAssets/Blueprints/Structures/ItemStruct Structure (by ref)"))
  (`KismetArrayLibrary.Array_Add` (`self.ArrayOfSlots`) NewItem)
  (return))

(fn `AddItemToEmptySlot`
  (params (Index :type Integer) (Item :type "/Game/MainAssets/Blueprints/Structures/ItemStruct Structure (by ref)"))
  (`KismetArrayLibrary.Array_Set` (`self.ArrayOfSlots`) Index Item)
  (return))

(fn `AddItemToStorage`
  (params (ItemInfo :type "/Game/MainAssets/Blueprints/Structures/ItemStruct Structure"))
  (returns (Success :type Boolean))
  (locals (L_ItemInfo :type "/Game/MainAssets/Blueprints/Structures/ItemStruct Structure") (L_SlotIndex :type Integer) (L_CanAddAmountToSlot :type Boolean :default false))
  (bind _l_iteminfo (`local.L_ItemInfo`))
  (bind ((`Name_24_B9821B4C44472B23BEDBA78B1411F5B8` _name) (`Amount_27_FC67A8E34DBED97F84EF428B5041EAB0` _amount)) (break `/Game/MainAssets/Blueprints/Structures/ItemStruct` (`local.L_ItemInfo`)))
  (bind _output_get (set `local.L_ItemInfo` ItemInfo))
  (if (`.DoesStack_15_35644A1C4DE8337B441AC1AA5D320217` (break `/Game/MainAssets/Blueprints/Structures/ItemStruct` _output_get))
    (for (_array_element _array_index) (`self.ArrayOfSlots`)
      (set `local.L_SlotIndex` _array_index)
      (bind ((`Name_24_B9821B4C44472B23BEDBA78B1411F5B8` _name_2) (`Amount_27_FC67A8E34DBED97F84EF428B5041EAB0` _amount_2) (`MaxStack_28_F31804514E5AE35989D84184E0692F26` _maxstack)) (break `/Game/MainAssets/Blueprints/Structures/ItemStruct` _array_element))
      (if (`KismetTextLibrary.EqualEqual_TextText` _name_2 _name)
        (if (<= (+ _amount_2 _amount) _maxstack)
          (set `local.L_CanAddAmountToSlot` true)
          (break))))
    (if (`local.L_CanAddAmountToSlot`)
      (`self.AddAmountToItem` _l_iteminfo (`local.L_SlotIndex`) (`.Amount_27_FC67A8E34DBED97F84EF428B5041EAB0` (break `/Game/MainAssets/Blueprints/Structures/ItemStruct` _l_iteminfo)))
      (`self.UpdateAllSlots`)
      (return true)
      (elif (`self.bLimitSlots`)
        (bind (_bsuccess _l_slotindex1) (`self.SearchForEmptySlot`))
        (if _bsuccess
          (`self.AddItemToEmptySlot` _l_slotindex1 (`local.L_ItemInfo`))
          (`self.UpdateAllSlots`)
          (return true))
        (else
          (return false))))
    (else
      (bind (_bsuccess_2 _l_slotindex1_2) (`self.SearchForEmptySlot`))
      (if _bsuccess_2
        (`self.AddItemToEmptySlot` _l_slotindex1_2 (`local.L_ItemInfo`))
        (`self.UpdateAllSlots`)
        (return true)))))

(fn `AddToExistingItem`
  (params (TheDraggedItemInfo :type "/Game/MainAssets/Blueprints/Structures/ItemStruct Structure") (TheDraggedItemIndex :type Integer) (CurrentItemInfo :type "/Game/MainAssets/Blueprints/Structures/ItemStruct Structure") (CurrentSlotIndex :type Integer))
  (locals (L_DraggedIn :type "/Game/MainAssets/Blueprints/Structures/ItemStruct Structure") (L_DraggedInIndex :type Integer) (L_CurrentInfo :type "/Game/MainAssets/Blueprints/Structures/ItemStruct Structure") (L_CurrentIndex :type Integer) (L_DraggedInAmount :type Integer) (L_TotalAmount :type Integer :default 0) (L_RemainingAmountToAdd :type Integer :default 0))
  (bind ((`Amount_27_FC67A8E34DBED97F84EF428B5041EAB0` _amount) (`MaxStack_28_F31804514E5AE35989D84184E0692F26` _maxstack)) (break `/Game/MainAssets/Blueprints/Structures/ItemStruct` (`local.L_CurrentInfo`)))
  (set `local.L_DraggedIn` TheDraggedItemInfo)
  (set `local.L_DraggedInIndex` TheDraggedItemIndex)
  (set `local.L_CurrentInfo` CurrentItemInfo)
  (set `local.L_CurrentIndex` CurrentSlotIndex)
  (bind _output_get (set `local.L_DraggedInAmount` (`.Amount_27_FC67A8E34DBED97F84EF428B5041EAB0` (break `/Game/MainAssets/Blueprints/Structures/ItemStruct` (`local.L_DraggedIn`)))))
  (bind _returnvalue (+ _output_get _amount))
  (bind _output_get_2 (set `local.L_TotalAmount` _returnvalue))
  (if (<= _returnvalue _maxstack)
    (`self.AddAmountToItem` (`local.L_CurrentInfo`) (`local.L_CurrentIndex`) (`.Amount_27_FC67A8E34DBED97F84EF428B5041EAB0` (break `/Game/MainAssets/Blueprints/Structures/ItemStruct` (`local.L_DraggedIn`))))
    (`self.RemoveItemFromSlot` (`local.L_DraggedInIndex`))
    (`self.UpdateAllSlots`)
    (`KismetSystemLibrary.PrintString` "Item Added")
    (return)
    (else
      (set `local.L_RemainingAmountToAdd` (- _output_get_2 _maxstack))
      (`self.AddAmountToItem` (`local.L_CurrentInfo`) (`local.L_CurrentIndex`) (- (- (`local.L_TotalAmount`) (`local.L_RemainingAmountToAdd`)) (`.Amount_27_FC67A8E34DBED97F84EF428B5041EAB0` (break `/Game/MainAssets/Blueprints/Structures/ItemStruct` (`local.L_CurrentInfo`)))))
      (`self.RemoveAmountFromSlot` (`local.L_DraggedIn`) (`local.L_DraggedInIndex`) (- (`local.L_DraggedInAmount`) (`local.L_RemainingAmountToAdd`)))
      (`self.UpdateAllSlots`)
      (return))))

(fn `DisplayAnItemBeingAdded`
  (params (ItemInfo :type "/Game/MainAssets/Blueprints/Structures/ItemStruct Structure"))
  (bind _returnvalue (`|CreateWidget` "/Game/MainAssets/Blueprints/Widgets/Widget_ShowAddItemVisual.Widget_ShowAddItemVisual_C" (`GameplayStatics.GetPlayerController` 0) ItemInfo))
  (`VerticalBox.AddChildToVerticalBox` (`/Game/MainAssets/Blueprints/Widgets/Widget_HUD_Inv.AddedItemBox` (`self.W_HUD`)) _returnvalue)
  (return))

(fn `GenerateSlots`
  (`PanelWidget.ClearChildren` (`/Game/MainAssets/Blueprints/Widgets/Widget_Storage.StorageSlots` (`self.W_StorageRef`)))
  (for (_array_element _array_index) (`self.ArrayOfSlots`)
    (bind _returnvalue (`|CreateWidget` "/Game/MainAssets/Blueprints/Widgets/Widget_StorageSlot.Widget_StorageSlot_C" null _array_element _array_index))
    (`WrapBox.AddChildToWrapBox` (`/Game/MainAssets/Blueprints/Widgets/Widget_Storage.StorageSlots` (`self.W_StorageRef`)) _returnvalue))
  (return))

(fn `InventorySetup`
  (if (`self.bLimitSlots`)
    (bind _result (`/Engine/EditorBlueprintResources/StandardMacros.DecrementInt` (`self.AmountOfSlots`))
      (:`  `
        (for _ (range (+ _result 1))
          (`KismetArrayLibrary.Array_Add` (`self.ArrayOfSlots`) (make `/Game/MainAssets/Blueprints/Structures/ItemStruct` "" null 0.0 0 false false 0 false true)))
        (return)))
    (else
      (return))))

(fn `OpenCloseInventory`
  (bind _returnvalue (`GameplayStatics.GetPlayerController` 0))
  (bind _w_storageref (`self.W_StorageRef`))
  (if (`self.bIsInventoryOpen`)
    (`Widget.RemoveFromParent` _w_storageref)
    (bind _output_get (set `self.bIsInventoryOpen` false))
    (set `PlayerController.bShowMouseCursor` _output_get _returnvalue)
    (`WidgetBlueprintLibrary.SetInputMode_GameOnly` _returnvalue)
    (else
      (`UserWidget.AddToViewport` _w_storageref 0)
      (set `self.bIsInventoryOpen` true)
      (set `PlayerController.bShowMouseCursor` true _returnvalue)
      (`self.GenerateSlots`)
      (`self.UpdateAllSlots`)
      (`WidgetBlueprintLibrary.SetInputMode_GameAndUIEx` _returnvalue (`self.W_StorageRef`)))))

(fn `RemoveAmountFromSlot`
  (params (ItemInfo :type "/Game/MainAssets/Blueprints/Structures/ItemStruct Structure") (SlotIndex :type Integer) (AmountToRemove :type Integer))
  (bind (_name _icon _weight _amount _edibleusable _doesexpire _maxstack _doesstack _emptyslot _description _healthofitem _enumtype) (break `/Game/MainAssets/Blueprints/Structures/ItemStruct` ItemInfo))
  (`KismetArrayLibrary.Array_Set` (`self.ArrayOfSlots`) SlotIndex (make `/Game/MainAssets/Blueprints/Structures/ItemStruct` _name _icon _weight (- _amount AmountToRemove) _edibleusable _doesexpire _maxstack _doesstack _emptyslot _description _healthofitem _enumtype)))

(fn `RemoveItemFromSlot`
  (params (IndexToRemove :type Integer))
  (bind _arrayofslots (`self.ArrayOfSlots`))
  (`KismetArrayLibrary.Array_Remove` _arrayofslots IndexToRemove)
  (`KismetArrayLibrary.Array_Add` _arrayofslots (make `/Game/MainAssets/Blueprints/Structures/ItemStruct` "" null 0.0 0 false false 0 false true))
  (`self.UpdateAllSlots`)
  (return))

(fn `RemoveItemFromSlotAndSpawnOnGround`
  (params (IndexToRemove :type Integer))
  (locals (L_Amount :type Integer) (L_EnumType :type "/Game/MainAssets/Blueprints/Enums/Enum_Pickup Enum"))
  (bind _arrayofslots (`self.ArrayOfSlots`))
  (bind _returnvalue (`Controller.K2_GetPawn` (`GameplayStatics.GetPlayerController` 0)))
  (bind ((`Amount_27_FC67A8E34DBED97F84EF428B5041EAB0` _amount) (`EnumType_31_1670885A408965D04ABA14BE39E2FDC7` _enumtype)) (break `/Game/MainAssets/Blueprints/Structures/ItemStruct` (`|GetArrayItem` (`self.ArrayOfSlots`) IndexToRemove)))
  (bind (_returnvalue_x _returnvalue_y _returnvalue_z) (`KismetMathLibrary.BreakVector` (+ (`Actor.K2_GetActorLocation` _returnvalue) (* (`Actor.GetActorForwardVector` _returnvalue) 300.0))))
  (set `local.L_Amount` _amount)
  (set `local.L_EnumType` _enumtype)
  (`KismetArrayLibrary.Array_Remove` _arrayofslots IndexToRemove)
  (`KismetArrayLibrary.Array_Add` _arrayofslots (make `/Game/MainAssets/Blueprints/Structures/ItemStruct` "" null 0.0 0 false false 0 false true))
  (`self.UpdateAllSlots`)
  (bind _result (`/Engine/EditorBlueprintResources/StandardMacros.DecrementInt` (`local.L_Amount`))
    (:`  `
      (for _ (range (+ _result 1))
        (`|SpawnActorFromClass` "/Game/MainAssets/Blueprints/Player_BPs/BP_MasterPickup.BP_MasterPickup_C" (`KismetMathLibrary.MakeTransform` (`KismetMathLibrary.MakeVector` _returnvalue_x _returnvalue_y (`KismetMathLibrary.RandomFloatInRange` (- _returnvalue_z -50.0) (+ _returnvalue_z 100.0)))) "AdjustIfPossibleButAlwaysSpawn" "OverrideRootScale" null (`local.L_EnumType`) null))
      (return))))

(fn `SearchForEmptySlot`
  (returns (bSuccess :type Boolean) (L_SlotIndex1 :type Integer))
  (locals (L_FoundEmptySlot :type Boolean) (L_SlotIndex :type Integer))
  (for (_array_element _array_index) (`self.ArrayOfSlots`)
    (set `local.L_SlotIndex` _array_index)
    (if (`.EmptySlot_17_946AC1534E363B36DE3546889DAADCE0` (break `/Game/MainAssets/Blueprints/Structures/ItemStruct` _array_element))
      (set `local.L_FoundEmptySlot` true)
      (break)))
  (if (`local.L_FoundEmptySlot`)
    (return true (`local.L_SlotIndex`))
    (else
      (return false 0))))

(fn `SplitStack`
  (params (ItemInfo :type "/Game/MainAssets/Blueprints/Structures/ItemStruct Structure") (SlotIndex :type Integer))
  (returns (bSuccess :type Boolean))
  (locals (L_ItemInfo :type "/Game/MainAssets/Blueprints/Structures/ItemStruct Structure") (L_SlotIndex :type Integer))
  (bind (_name _icon _weight _amount _edibleusable _doesexpire _maxstack _doesstack _emptyslot _description _healthofitem _enumtype) (break `/Game/MainAssets/Blueprints/Structures/ItemStruct` (`local.L_ItemInfo`)))
  (bind _returnvalue (/ _amount 2))
  (bind _output_get (set `local.L_ItemInfo` ItemInfo))
  (set `local.L_SlotIndex` SlotIndex)
  (if (> (`.Amount_27_FC67A8E34DBED97F84EF428B5041EAB0` (break `/Game/MainAssets/Blueprints/Structures/ItemStruct` _output_get)) 1)
    (bind (_bsuccess _l_slotindex1) (`self.SearchForEmptySlot`))
    (if _bsuccess
      (`self.AddItemToEmptySlot` _l_slotindex1 (make `/Game/MainAssets/Blueprints/Structures/ItemStruct` _name _icon _weight _returnvalue _edibleusable _doesexpire _maxstack _doesstack _emptyslot _description _healthofitem _enumtype))
      (`self.RemoveAmountFromSlot` (`local.L_ItemInfo`) (`local.L_SlotIndex`) _returnvalue)
      (`self.UpdateAllSlots`)
      (return true)
      (elif (`self.bLimitSlots`)
        (`KismetSystemLibrary.PrintString` "Not Enough Space")
        (return false)
        (else
          (`self.AddItemToArray` (`local.L_ItemInfo`))
          (return true))))
    (else
      (return false))))

(fn `SwapItemIndex`
  (params (TheDraggedItemInfo :type "/Game/MainAssets/Blueprints/Structures/ItemStruct Structure") (TheDraggedItemIndex :type Integer) (CurrentItemInfo :type "/Game/MainAssets/Blueprints/Structures/ItemStruct Structure") (CurrentSlotIndex :type Integer))
  (`KismetArrayLibrary.Array_Set` (`self.ArrayOfSlots`) CurrentSlotIndex TheDraggedItemInfo)
  (`KismetArrayLibrary.Array_Set` (`self.ArrayOfSlots`) TheDraggedItemIndex CurrentItemInfo)
  (`self.UpdateAllSlots`)
  (return))

(fn `UpdateAllSlots`
  (for (_array_element _array_index) (`self.ArrayOfSlots`)
    (bind _aswidget_storage_slot (cast `/Game/MainAssets/Blueprints/Widgets/Widget_StorageSlot` (`PanelWidget.GetChildAt` (`/Game/MainAssets/Blueprints/Widgets/Widget_Storage.StorageSlots` (`self.W_StorageRef`)) _array_index)))
    (`/Game/MainAssets/Blueprints/Widgets/Widget_StorageSlot.UpdateSlotInfo` _aswidget_storage_slot _array_element))
  (return))