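; Master pickup actor that represents every inventory item type, from food and potions to crafting materials and wooden foundations, selected by the EnumPickup variable.
; The construction script switches on that enum and calls a per-item graph that sets the static mesh and, if that succeeds, fills the ItemInfo struct.
; Wooden foundations also set a Structure flag; on BeginPlay, anything not flagged enables mesh physics after a one-second delay.
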(event `self.ReceiveBeginPlay`
  (`KismetSystemLibrary.Delay` 1.0)
  (if (not (`self.Structure`))
    (`PrimitiveComponent.SetSimulatePhysics` (`self.StaticMesh`) true)))

(fn `UserConstructionScript`
  (switch `/Game/MainAssets/Blueprints/Enums/Enum_ItemType` (`self.Enum_Pickup`)
    (:`NewEnumerator0`
      (bind _returnvalue (`StaticMeshComponent.SetStaticMesh` (`self.StaticMesh`) "/Game/Placeholder_Meshes/SM_Food.SM_Food"))
      (if _returnvalue
        (set `self.ItemInfo` (make `/Game/MainAssets/Blueprints/Structures/ItemStruct` "Food" "/Game/Placeholder_Meshes/Images/T_Food.T_Food" 0.1 1 true true 25 true false "Whatever the heart desires" 100.0 (`self.Enum_Pickup`) (`self.SlotType`)))))
    (:`NewEnumerator1`
      (bind _returnvalue_2 (`StaticMeshComponent.SetStaticMesh` (`self.StaticMesh`) "/Game/Placeholder_Meshes/SM_ManaPotion.SM_ManaPotion"))
      (if _returnvalue_2
        (set `self.ItemInfo` (make `/Game/MainAssets/Blueprints/Structures/ItemStruct` "Mana Potion" "/Game/Placeholder_Meshes/Images/T_Mana.T_Mana" 0.2 1 true true 20 true false "To restore mana for Oarf" 100.0 (`self.Enum_Pickup`) (`self.SlotType`)))))
    (:`NewEnumerator2`
      (bind _returnvalue_3 (`StaticMeshComponent.SetStaticMesh` (`self.StaticMesh`) "/Game/Placeholder_Meshes/SM_HealthPotion.SM_HealthPotion"))
      (if _returnvalue_3
        (set `self.ItemInfo` (make `/Game/MainAssets/Blueprints/Structures/ItemStruct` "HealthPotion" "/Game/Placeholder_Meshes/Images/T_HealthPotion.T_HealthPotion" 0.2 1 true false 20 true false "Health Potion for Oarf" 100.0 (`self.Enum_Pickup`) (`self.SlotType`)))))
    (:`NewEnumerator3`
      (bind _returnvalue_4 (`StaticMeshComponent.SetStaticMesh` (`self.StaticMesh`) "/Game/Placeholder_Meshes/SM_Sticks.SM_Sticks"))
      (if _returnvalue_4
        (set `self.ItemInfo` (make `/Game/MainAssets/Blueprints/Structures/ItemStruct` "Sticks" "/Game/Placeholder_Meshes/Images/T_Sticks.T_Sticks" 0.5 5 false false 25 true false "Sticks, not stones." 100.0 (`self.Enum_Pickup`) (`self.SlotType`)))))
    (:`NewEnumerator4`
      (bind _returnvalue_5 (`StaticMeshComponent.SetStaticMesh` (`self.StaticMesh`) "/Game/Placeholder_Meshes/SM_Wood.SM_Wood"))
      (if _returnvalue_5
        (set `self.ItemInfo` (make `/Game/MainAssets/Blueprints/Structures/ItemStruct` "Wood" "/Game/Placeholder_Meshes/Images/T_Wood.T_Wood" 2.0 1 false false 10 true false "Better Use Some Protection." 100.0 (`self.Enum_Pickup`) (`self.SlotType`)))))
    (:`NewEnumerator5`
      (bind _returnvalue_6 (`StaticMeshComponent.SetStaticMesh` (`self.StaticMesh`) "/Game/Placeholder_Meshes/SM_Plank.SM_Plank"))
      (if _returnvalue_6
        (set `self.ItemInfo` (make `/Game/MainAssets/Blueprints/Structures/ItemStruct` "Planks" "/Game/Placeholder_Meshes/Images/T_Plank.T_Plank" 1.0 1 true false 5 true false "Walking along these can lead to serious injury or death." 100.0 (`self.Enum_Pickup`) (`self.SlotType`)))))
    (:`NewEnumerator6`
      (bind _returnvalue_7 (`StaticMeshComponent.SetStaticMesh` (`self.StaticMesh`) "/Game/Placeholder_Meshes/SM_Stone.SM_Stone"))
      (if _returnvalue_7
        (set `self.ItemInfo` (make `/Game/MainAssets/Blueprints/Structures/ItemStruct` "Stone" "/Game/Placeholder_Meshes/Images/T_Stone.T_Stone" 2.0 1 true false 5 true false "Medkit, not for eating" 100.0 (`self.Enum_Pickup`) (`self.SlotType`)))))
    (:`NewEnumerator7`
      (bind _returnvalue_8 (`StaticMeshComponent.SetStaticMesh` (`self.StaticMesh`) "/Game/Placeholder_Meshes/SM_Iron.SM_Iron"))
      (if _returnvalue_8
        (set `self.ItemInfo` (make `/Game/MainAssets/Blueprints/Structures/ItemStruct` "Iron" "/Game/Placeholder_Meshes/Images/T_Iron.T_Iron" 5.0 1 true false 5 true false "Tough Stuff" 100.0 (`self.Enum_Pickup`) (`self.SlotType`)))))
    (:`NewEnumerator8`
      (bind _returnvalue_9 (`StaticMeshComponent.SetStaticMesh` (`self.StaticMesh`) "/Game/Placeholder_Meshes/SM_Steel.SM_Steel"))
      (if _returnvalue_9
        (set `self.ItemInfo` (make `/Game/MainAssets/Blueprints/Structures/ItemStruct` "Steel" "/Game/Placeholder_Meshes/Images/T_Steel.T_Steel" 5.0 1 true false 5 true false "Man Not Included." 100.0 (`self.Enum_Pickup`) (`self.SlotType`)))))
    (:`NewEnumerator9`
      (bind _returnvalue_10 (`StaticMeshComponent.SetStaticMesh` (`self.StaticMesh`) "/Game/Placeholder_Meshes/SM_Cloth.SM_Cloth"))
      (if _returnvalue_10
        (set `self.ItemInfo` (make `/Game/MainAssets/Blueprints/Structures/ItemStruct` "Cloth" "/Game/Placeholder_Meshes/Images/T_Cloth.T_Cloth" 0.5 1 true false 25 true false "Not invisible, so you don't need to worry." 100.0 (`self.Enum_Pickup`) (`self.SlotType`)))))
    (:`NewEnumerator10`
      (bind _returnvalue_11 (`StaticMeshComponent.SetStaticMesh` (`self.StaticMesh`) "/Game/Placeholder_Meshes/SM_AnimalSkin.SM_AnimalSkin"))
      (if _returnvalue_11
        (set `self.ItemInfo` (make `/Game/MainAssets/Blueprints/Structures/ItemStruct` "Leather" "/Game/Placeholder_Meshes/Images/T_AnimalSkin.T_AnimalSkin" 1.0 1 true false 10 true false "Purchased From Florida Mortuaries." 100.0 (`self.Enum_Pickup`) (`self.SlotType`)))))
    (:`NewEnumerator11`
      (bind _returnvalue_12 (`StaticMeshComponent.SetStaticMesh` (`self.StaticMesh`) "/Game/Placeholder_Meshes/SM_AnimalSkin.SM_AnimalSkin"))
      (if _returnvalue_12
        (set `self.ItemInfo` (make `/Game/MainAssets/Blueprints/Structures/ItemStruct` "Animal Skin" "/Game/Placeholder_Meshes/Images/T_AnimalSkin.T_AnimalSkin" 1.0 1 true false 10 true false "" 100.0 (`self.Enum_Pickup`) (`self.SlotType`)))))
    (:`NewEnumerator12`
      (bind _returnvalue_13 (`StaticMeshComponent.SetStaticMesh` (`self.StaticMesh`) "/Game/Placeholder_Meshes/SM_HornsMagazine.SM_HornsMagazine"))
      (if _returnvalue_13
        (set `self.ItemInfo` (make `/Game/MainAssets/Blueprints/Structures/ItemStruct` "Horns Magazine" "/Game/Placeholder_Meshes/Images/T_Horns.T_Horns" 0.2 1 true false 25 true false "For The Gentleman From Every Species" 100.0 (`self.Enum_Pickup`) (`self.SlotType`)))))
    (:`NewEnumerator13`
      (bind _returnvalue_14 (`StaticMeshComponent.SetStaticMesh` (`self.StaticMesh`) "/Game/Placeholder_Meshes/SM_Nails.SM_Nails"))
      (if _returnvalue_14
        (set `self.ItemInfo` (make `/Game/MainAssets/Blueprints/Structures/ItemStruct` "Nails" "/Game/Placeholder_Meshes/Images/T_Nails.T_Nails" 0.2 1 true false 100 true false "" 100.0 (`self.Enum_Pickup`) (`self.SlotType`)))))
    (:`NewEnumerator15`
      (bind _returnvalue_15 (`StaticMeshComponent.SetStaticMesh` (`self.StaticMesh`) "/Game/MainAssets/Buildings/Meshes/Foundations/Foundation_200x200_01_x.Foundation_200x200_01_x"))
      (if _returnvalue_15
        (set `self.ItemInfo` (make `/Game/MainAssets/Blueprints/Structures/ItemStruct` "Foundation 2x2" "/Game/HUD/Textures/Dot.Dot" 0.0 1 true false 25 true false "Whatever the heart desires" 100.0 (`self.Enum_Pickup`) (`self.SlotType`)))
        (set `self.Structure` true)))))