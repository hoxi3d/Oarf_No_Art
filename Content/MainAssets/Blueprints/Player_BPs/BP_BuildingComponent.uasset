(event `self.ReceiveTick`
  (params (DeltaSeconds :type "Float (single-precision)"))
  (bind _oarfcontrollerref (`self.OarfControllerRef`))
  (bind _returnvalue (`Actor.K2_GetActorLocation` (`Controller.K2_GetPawn` _oarfcontrollerref)))
  (`/Engine/EditorBlueprintResources/StandardMacros.IsValid` _oarfcontrollerref
    (:`Is Valid`
      (if (`self.BuildMode`)
        (`KismetSystemLibrary.PrintString` "Build Mode On" true true (struct :`G` 0.66 :`B` 1.0 :`A` 1.0) 0.01)
        (bind (_outhit _returnvalue_2) (`KismetSystemLibrary.LineTraceSingleForObjects` :`Start` _returnvalue :`End` (+ _returnvalue (* (`KismetMathLibrary.Conv_RotatorToVector` (`Controller.GetControlRotation` _oarfcontrollerref)) 1000.0)) :`ObjectTypes` (`|MakeArray` "ObjectTypeQuery2" "ObjectTypeQuery8" :!type "EObjectTypeQuery Enum") :`DrawDebugType` "ForOneFrame" :`DrawTime` 1.0 :!label _label))
        (if _returnvalue_2
          (bind (_bblockinghit _binitialoverlap _time _distance _location _impactpoint _normal _impactnormal _physmat _hitactor) (`GameplayStatics.BreakHitResult` _outhit))
          (bind _output_get (set `self.LineTraceHitLocation` _location))
          (bind _asbp_master_pickup (cast `/Game/MainAssets/Blueprints/Player_BPs/BP_MasterPickup` _hitactor)
            (:`then`
              (if (`/Game/MainAssets/Blueprints/Player_BPs/BP_MasterPickup.Structure` _asbp_master_pickup)
                (if (`self.BuildMode`)
                  (set `self.As BP Master Pickup` _asbp_master_pickup)
                  (`KismetSystemLibrary.PrintString` (`KismetStringLibrary.Concat_StrStr` "CastWorked \nSet AsBPMasterPickup" (`KismetStringLibrary.Conv_VectorToString` _output_get)) true true (struct :`G` 0.66 :`B` 1.0 :`A` 1.0) 0.01)
                  (elif (`/Game/MainAssets/Blueprints/Player_BPs/BP_MasterPickup.Built` _asbp_master_pickup)
                    _))))
            (:`CastFailed`
              (set `self.CurrentLookAtItem` null :!label _label_2)))
          (else
            (goto _label_2)))))
    (:`Is Not Valid`
      (goto _label))))

(event `Build`
  (params (CraftItemInfo :type "/Game/MainAssets/Blueprints/Structures/CraftRecipes Structure") (ItemType :type "/Game/MainAssets/Blueprints/Enums/Enum_ItemType Enum" :default "NewEnumerator14"))
  (bind _oarfcontrollerref (`self.OarfControllerRef`))
  (if (`/Game/MainAssets/Blueprints/Player_BPs/BP_Oarf.IsWeaponEquipped` (`self. BPOarfRef`))
    (set `self.BuildMode` true)
    (bind _output_get (set `self.CraftItemInfo` CraftItemInfo))
    (bind _output_get_2 (set `self.ItemType` ItemType))
    (bind _issnapping (`self.SnapBuilding`))
    (if _issnapping
      (`KismetSystemLibrary.PrintString` "Snapping = Good")
      (bind _snaptype (`self.FindSnapCategory`))
      (switch `/Game/MainAssets/Blueprints/Enums/Enum_SnapType` _snaptype
        (:`NewEnumerator0`
          (`KismetSystemLibrary.PrintString` "SwitchGood")
          (`self.SnapFoundation`)
          (`KismetSystemLibrary.PrintString` "SnapGood")
          (`self.SetTransform` true)
          (bind _returnvalue (`self.SpawnTempActor`))
          (`KismetSystemLibrary.Delay` 0.1)
          (`self.AskToPlaceItemOrCancelBuildMode` _returnvalue)))
      (else
        (bind _returnvalue_2 (`|SpawnActorFromClass` "/Game/MainAssets/Blueprints/Player_BPs/BP_MasterPickup.BP_MasterPickup_C" (`KismetMathLibrary.MakeTransform` (`self.LineTraceHitLocation`)) "AlwaysSpawn" "OverrideRootScale" null _output_get_2 false null))
        (bind _staticmesh (`/Game/MainAssets/Blueprints/Player_BPs/BP_MasterPickup.StaticMesh` _returnvalue_2))
        (`PrimitiveComponent.SetCollisionEnabled` _staticmesh "NoCollision")
        (`PrimitiveComponent.SetMaterial` _staticmesh 0 "/Game/MainAssets/Materials/MI_Color_Green.MI_Color_Green")
        (`KismetSystemLibrary.Delay` 0.1)
        (`Actor.K2_DestroyActor` _returnvalue_2)
        (if (`/Game/MainAssets/Blueprints/Player_BPs/BP_Oarf_Controller.BuildModeCancelConstruction` _oarfcontrollerref)
          (set `self.BuildMode` false)
          (elif (`/Game/MainAssets/Blueprints/Player_BPs/BP_Oarf_Controller.BuildModeFlopper` _oarfcontrollerref)
            (`|SpawnActorFromClass` "/Game/MainAssets/Blueprints/Player_BPs/BP_MasterPickup.BP_MasterPickup_C" (`KismetMathLibrary.MakeTransform` (`self.LineTraceHitLocation`)) "Undefined" "OverrideRootScale" null (`self.ItemType`) false null)
            (set `self.BuildMode` false)
            (else
              (`self.Build` (`self.CraftItemInfo`) "NewEnumerator15"))))))))

(fn `AskToPlaceItemOrCancelBuildMode`
  (params (CurrentLookAtItem :type "/Game/MainAssets/Blueprints/Player_BPs/BP_MasterPickup Object Reference"))
  (bind __bpoarfref (`self. BPOarfRef`))
  (if (`/Game/MainAssets/Blueprints/Player_BPs/BP_Oarf.RMBDown` __bpoarfref)
    (`Actor.K2_DestroyActor` CurrentLookAtItem)
    (set `self.BuildMode` false)
    (`KismetSystemLibrary.PrintString` "CandelBuild")
    (elif (`/Game/MainAssets/Blueprints/Player_BPs/BP_Oarf.LMBDown` __bpoarfref)
      (`Actor.K2_DestroyActor` CurrentLookAtItem)
      (`|SpawnActorFromClass` "/Game/MainAssets/Blueprints/Player_BPs/BP_MasterPickup.BP_MasterPickup_C" (`self.SpawnTransformation`) "Undefined" "OverrideRootScale" null (`self.ItemType`) true null)
      (set `self.BuildMode` false)
      (else
        (`Actor.K2_DestroyActor` CurrentLookAtItem)
        (`self.Build` (`self.CraftItemInfo`) (`self.ItemType`))))))

(fn `FindSnapCategory`
  (returns (SnapType :type "/Game/MainAssets/Blueprints/Enums/Enum_SnapType Enum"))
  (bind _returnvalue (`|SpawnActorFromClass` "/Game/MainAssets/Blueprints/Player_BPs/BP_MasterPickup.BP_MasterPickup_C" (`KismetMathLibrary.MakeTransform` (0.0 0.0 10000000.0)) "Undefined" "OverrideRootScale" null (`self.ItemType`) false null))
  (bind _output_get (set `self.SnapType` (`.SnapType_38_6022441F4DB880B5B42DA492BEC46FBE` (break `/Game/MainAssets/Blueprints/Structures/ItemStruct` (`/Game/MainAssets/Blueprints/Player_BPs/BP_MasterPickup.ItemInfo` _returnvalue)))))
  (`Actor.K2_DestroyActor` _returnvalue)
  (`KismetSystemLibrary.PrintString` "Snap Category Found")
  (return _output_get))

(fn `SetTransform`
  (params (Snap :type Boolean))
  (bind _currentlookatitem (`self.CurrentLookAtItem`))
  (`/Engine/EditorBlueprintResources/StandardMacros.IsValid` _currentlookatitem
    (:`Is Valid`
      (if Snap
        (bind _output_get (set `self.SpawnTransformation` (`KismetMathLibrary.MakeTransform` (+ (`SceneComponent.K2_GetComponentLocation` (`/Game/MainAssets/Blueprints/Player_BPs/BP_MasterPickup.StaticMesh` _currentlookatitem)) (.location (`self.SnapOffset`))) (.rotation (`self.SnapOffset`)))))
        (`KismetSystemLibrary.PrintString` (`KismetStringLibrary.Conv_TransformToString` _output_get))
        (return)))))

(fn `SnapBuilding`
  (returns (IsSnapping :type Boolean))
  (`/Engine/EditorBlueprintResources/StandardMacros.IsValid` (`self.CurrentLookAtItem`)
    (:`Is Valid`
      (`KismetSystemLibrary.PrintString` "Valid Snap Building" true true (struct :`G` 0.66 :`B` 1.0 :`A` 1.0) 0.1)
      (return (`/Game/MainAssets/Blueprints/Player_BPs/BP_Oarf.IsSnapping` (`self. BPOarfRef`))))
    (:`Is Not Valid`
      (`KismetSystemLibrary.PrintString` "Not Valid Snap Building" true true (struct :`G` 0.66 :`B` 1.0 :`A` 1.0) 0.01)
      (return false))))

(fn `SnapFoundation`
  (bind _location (.location (`SceneComponent.K2_GetComponentToWorld` (`/Game/MainAssets/Blueprints/Player_BPs/BP_MasterPickup.StaticMesh` (`self.CurrentLookAtItem`)))))
  (bind _returnvalue (- _location (`self.LineTraceHitLocation`)))
  (`KismetSystemLibrary.PrintString` (`KismetStringLibrary.Conv_VectorToString` _location))
  (if (== (`KismetMathLibrary.MakeVector` (.x _returnvalue) (.y _returnvalue)) (100.0 0.0 0.0) :`ErrorTolerance` 60.0)
    (`KismetSystemLibrary.PrintString` "Up")
    (set `self.SnapOffset` (`KismetMathLibrary.MakeTransform` (-200.0 0.0 0.0)))
    (return)
    (elif (== (`KismetMathLibrary.MakeVector` (.x _returnvalue) (.y _returnvalue)) (0.0 100.0 0.0) :`ErrorTolerance` 60.0)
      (`KismetSystemLibrary.PrintString` "Right")
      (set `self.SnapOffset` (`KismetMathLibrary.MakeTransform` (0.0 -200.0 0.0)))
      (return)
      (elif (== (`KismetMathLibrary.MakeVector` (.x _returnvalue) (.y _returnvalue)) (-100.0 0.0 0.0) :`ErrorTolerance` 60.0)
        (`KismetSystemLibrary.PrintString` "Down")
        (set `self.SnapOffset` (`KismetMathLibrary.MakeTransform` (200.0 0.0 0.0)))
        (return)
        (elif (== (`KismetMathLibrary.MakeVector` (.x _returnvalue) (.y _returnvalue)) (0.0 -100.0 0.0) :`ErrorTolerance` 60.0)
          (`KismetSystemLibrary.PrintString` "Left")
          (set `self.SnapOffset` (`KismetMathLibrary.MakeTransform` (0.0 200.0 0.0)))
          (return)
          (else
            (`KismetSystemLibrary.PrintString` "No Snap Found")))))))

(fn `SpawnTempActor`
  (returns (ReturnValue :type "/Game/MainAssets/Blueprints/Player_BPs/BP_MasterPickup Object Reference"))
  (bind _returnvalue (`|SpawnActorFromClass` "/Game/MainAssets/Blueprints/Player_BPs/BP_MasterPickup.BP_MasterPickup_C" (`self.SpawnTransformation`) "Undefined" "OverrideRootScale" null (`self.ItemType`) false null))
  (bind _staticmesh (`/Game/MainAssets/Blueprints/Player_BPs/BP_MasterPickup.StaticMesh` _returnvalue))
  (`PrimitiveComponent.SetCollisionEnabled` _staticmesh "NoCollision")
  (`PrimitiveComponent.SetMaterial` _staticmesh 0 "/Game/MainAssets/Materials/MI_Color_Green.MI_Color_Green")
  (return _returnvalue))