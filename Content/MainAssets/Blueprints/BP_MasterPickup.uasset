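; BP_MasterPickup is a pickup item whose type (Apple, Watermelon or Medkit) is selected by the EnumPickup variable.
; The Construction Script switches on that enum to set a basic shape mesh, then fills ItemInfo with a name and shared icon only if the mesh call returns true.
; One second after BeginPlay it turns off physics simulation on the mesh.
; It contains no overlap or collection logic.
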(event `self.ReceiveBeginPlay`
  (`KismetSystemLibrary.Delay` 1.0)
  (`PrimitiveComponent.SetSimulatePhysics` (`self.StaticMesh`) false))

(fn `UserConstructionScript`
  (switch `/Game/MainAssets/Blueprints/Enums/Enum_Pickup` (`self.Enum_Pickup`)
    (:`NewEnumerator0`
      (bind _returnvalue (`StaticMeshComponent.SetStaticMesh` (`self.StaticMesh`) "/Game/MainAssets/Buildings/Meshes/Ramps/Ramp_100x100x100_01_x.Ramp_100x100x100_01_x"))
      (if _returnvalue
        (set `self.ItemInfo` (make `/Game/MainAssets/Blueprints/Structures/ItemStruct` "Apple" "/Game/HUD/MiniMap/Oarf.Oarf" 1.0 1 true true 25 true false "Apple" 100.0))))
    (:`NewEnumerator1`
      (bind _returnvalue_2 (`StaticMeshComponent.SetStaticMesh` (`self.StaticMesh`) "/Game/MainAssets/Buildings/Meshes/Floors/Floor_100x100_01_x.Floor_100x100_01_x"))
      (if _returnvalue_2
        (set `self.ItemInfo` (make `/Game/MainAssets/Blueprints/Structures/ItemStruct` "Watermelon" "/Game/HUD/MiniMap/Oarf.Oarf" 5.0 1 true true 5 true false "Watermelon for eating" 100.0 "NewEnumerator1"))))
    (:`NewEnumerator2`
      (bind _returnvalue_3 (`StaticMeshComponent.SetStaticMesh` (`self.StaticMesh`) "/Game/MainAssets/Buildings/Meshes/Foundations/Foundation_100x100_01_x.Foundation_100x100_01_x"))
      (if _returnvalue_3
        (set `self.ItemInfo` (make `/Game/MainAssets/Blueprints/Structures/ItemStruct` "Medkit" "/Game/HUD/MiniMap/Oarf.Oarf" 1.0 1 true false 10 true false "Medkit, not for eating" 100.0 "NewEnumerator2"))))))