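; Base quest actor that tracks which sub-goals of a quest are currently active.
; SetUpStartingGoals seeds the active index list from the starting indices, and UpdateSubGoals rebuilds the current goals from QuestInfo using those indices.
; GoToNextSubGoal replaces all active indices with the one after the highest, returning false when no sub-goal remains.
; The event graph is empty, so these functions run only when called.
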(fn `GoToNextSubGoal`
  (returns (Success :type Boolean))
  (locals (NextIndex :type Integer :default 0))
  (bind _currentgoalindeces (`self.CurrentGoalIndeces`))
  (bind _returnvalue (+ (`.MaxValue` (`KismetMathLibrary.MaxOfIntArray` (`self.CurrentGoalIndeces`))) 1))
  (if (<= _returnvalue (`KismetArrayLibrary.Array_LastIndex` (`.SubGoals_62_6663B5074689DF44D9D38688E643AB95` (break `/Game/HUD/Quests/Structs/Struct_QuestInfo` (`self.QuestInfo`)))))
    (set `local.NextIndex` _returnvalue)
    (`KismetArrayLibrary.Array_Clear` _currentgoalindeces)
    (`KismetArrayLibrary.Array_Add` _currentgoalindeces (`local.NextIndex`))
    (`self.UpdateSubGoals`)
    (return true)
    (else
      (return false))))

(fn `SetUpStartingGoals`
  (`KismetArrayLibrary.Array_Clear` (`self.CurrentGoalIndeces`))
  (set `self.CurrentGoalIndeces` (`self.StartingSubGoalIndeces`))
  (`self.UpdateSubGoals`)
  (return))

(fn `UpdateSubGoals`
  (`KismetArrayLibrary.Array_Clear` (`self.CurrentGoals`))
  (for _array_element (`self.CurrentGoalIndeces`)
    (`KismetArrayLibrary.Array_Add` (`self.CurrentGoals`) (`|GetArrayItem` (`.SubGoals_62_6663B5074689DF44D9D38688E643AB95` (break `/Game/HUD/Quests/Structs/Struct_QuestInfo` (`self.QuestInfo`))) _array_element)))
  (return))

(fn `UserConstructionScript`)