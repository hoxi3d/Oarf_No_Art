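; BP_GoalActor is a goal marker actor with minimap icon and radius sprite components.
; On BeginPlay it sets the first player character as its owner; the owner-no-see call is left unconnected.
; The construction script is empty, with disconnected logic that would toggle between icon and radius circle by UseRadius, then scale and tint the circle from Radius and CircleColor.
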(event `self.ReceiveBeginPlay`
  (`self.SetOwner` (`GameplayStatics.GetPlayerCharacter` 0)))

(fn `UserConstructionScript`)