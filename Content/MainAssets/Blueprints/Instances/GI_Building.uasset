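; GI_Building is a game instance Blueprint that tracks the current mesh variant index for each building class.
; A CurrentMeshIndex map stores one index per class, and GetMeshIndex reads it.
; IncrementMeshIndex advances that index, wraps it to zero on reaching the supplied mesh count, then stores and returns it, cycling through the variants.
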(fn `GetMeshIndex`
  (params (Class :type "/Game/MainAssets/Buildings/BPs/BP_Building_Base Class Reference"))
  (returns (Index :type Integer))
  (return (`BlueprintMapLibrary.Map_Find` (`self.CurrentMeshIndex`) Class)))

(fn `IncrementMeshIndex`
  (params (Class :type "/Game/MainAssets/Buildings/BPs/BP_Building_Base Class Reference") (NumberMesh :type Integer))
  (returns (NewIndex :type Integer))
  (locals (NextMeshIndex :type Integer :default 0))
  (bind _nextmeshindex (`local.NextMeshIndex`))
  (bind _output_get (set `local.NextMeshIndex` (+ (`BlueprintMapLibrary.Map_Find` (`self.CurrentMeshIndex`) Class) 1)))
  (if (>= _output_get NumberMesh)
    (set `local.NextMeshIndex` 0))
  (`BlueprintMapLibrary.Map_Add` (`self.CurrentMeshIndex`) (`local.Class`) _nextmeshindex)
  (return _nextmeshindex))